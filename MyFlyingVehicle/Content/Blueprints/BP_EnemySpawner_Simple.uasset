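; Simple enemy spawner that endlessly spawns one of two enemy Blueprints at random along a horizontal line.
; Two arrow components mark the Y range, with the right arrow also supplying X and Z, and each enemy spawns with a fixed rotation regardless of collision.
; A timer starts on BeginPlay and re-arms after every spawn with a new random delay of a few seconds.
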(event `self.ReceiveBeginPlay`
  (`KismetSystemLibrary.K2_SetTimerDelegate` (delegate `SpawnEnemy`) (`KismetMathLibrary.RandomFloatInRange` 2.0 4.0) false true :!label _label))

(event `SpawnEnemy`
  (bind (_returnvalue_x _returnvalue_y _returnvalue_z) (`KismetMathLibrary.BreakVector` (`SceneComponent.K2_GetComponentLocation` (`self.Arrow_Right`))))
  (bind (_returnvalue_x_2 _returnvalue_y_2) (`KismetMathLibrary.BreakVector` (`SceneComponent.K2_GetComponentLocation` (`self.Arrow_Left`))))
  (`|SpawnActorFromClass` (`KismetArrayLibrary.Array_Random` (`|MakeArray` "/Game/Blueprints/BP_Enemy_1.BP_Enemy_1_C" "/Game/Blueprints/BP_Enemy_2.BP_Enemy_2_C" :!type "Actor Class Reference")) (`KismetMathLibrary.MakeTransform` (`KismetMathLibrary.MakeVector` _returnvalue_x (`KismetMathLibrary.RandomFloatInRange` _returnvalue_y _returnvalue_y_2) _returnvalue_z) (struct :`Yaw` 180.0)) "AlwaysSpawn" "MultiplyWithRoot")
  (goto _label))

(fn `UserConstructionScript`)